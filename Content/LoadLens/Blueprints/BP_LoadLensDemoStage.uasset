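; LoadLens demo stage that loads six heavy textures one at a time onto six screens, either blocking or asynchronously.
; LoadNextBlocking and LoadNextAsync resolve the next texture's soft path via PathForIndex, and ApplyTexture sets it on that screen through a dynamic material instance.
; NextIndex advances after each successful load, which for async happens only on completion.
; ResetDemo restores the base screen material, resets LoadLens and forces garbage collection.
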(event `LoadNextBlocking`
  (bind _nextindex (`self.NextIndex`))
  (if (< _nextindex 6)
    (bind _path (`self.PathForIndex` _nextindex))
    (bind _returnvalue (`KismetSystemLibrary.LoadAsset_Blocking` (`KismetSystemLibrary.Conv_SoftObjPathToSoftObjRef` (`KismetSystemLibrary.MakeSoftObjectPath` _path))))
    (bind _astexture_2d (cast `Texture2D` _returnvalue))
    (`self.ApplyTexture` _nextindex _astexture_2d)
    (set `self.NextIndex` (+ _nextindex 1))))

(event `LoadNextAsync`
  (bind _nextindex (`self.NextIndex`))
  (if (< _nextindex 6)
    (bind _path (`self.PathForIndex` _nextindex))
    (bind _object (`|LoadAsset` (`KismetSystemLibrary.Conv_SoftObjPathToSoftObjRef` (`KismetSystemLibrary.MakeSoftObjectPath` _path)))
      (:`Completed`
        (bind _astexture_2d (cast `Texture2D` _object))
        (`self.ApplyTexture` _nextindex _astexture_2d)
        (set `self.NextIndex` (+ _nextindex 1))))))

(event `ResetDemo`
  (set `self.NextIndex` 0)
  (`PrimitiveComponent.SetMaterial` (`self.Screen1`) 0 "/LoadLens/LoadLens/Materials/M_LoadLensScreen.M_LoadLensScreen")
  (`PrimitiveComponent.SetMaterial` (`self.Screen2`) 0 "/LoadLens/LoadLens/Materials/M_LoadLensScreen.M_LoadLensScreen")
  (`PrimitiveComponent.SetMaterial` (`self.Screen3`) 0 "/LoadLens/LoadLens/Materials/M_LoadLensScreen.M_LoadLensScreen")
  (`PrimitiveComponent.SetMaterial` (`self.Screen4`) 0 "/LoadLens/LoadLens/Materials/M_LoadLensScreen.M_LoadLensScreen")
  (`PrimitiveComponent.SetMaterial` (`self.Screen5`) 0 "/LoadLens/LoadLens/Materials/M_LoadLensScreen.M_LoadLensScreen")
  (`PrimitiveComponent.SetMaterial` (`self.Screen6`) 0 "/LoadLens/LoadLens/Materials/M_LoadLensScreen.M_LoadLensScreen")
  (`LoadLensStatics.ResetLoadLens`)
  (`KismetSystemLibrary.CollectGarbage`))

(fn `ApplyTexture`
  (params (Index :type Integer) (Tex :type "Texture2D Object Reference"))
  (switch `int` Index
    (:`0`
      (bind _returnvalue (`PrimitiveComponent.CreateDynamicMaterialInstance` (`self.Screen1`) 0 null "None"))
      (`MaterialInstanceDynamic.SetTextureParameterValue` _returnvalue "BaseTexture" Tex))
    (:`1`
      (bind _returnvalue_2 (`PrimitiveComponent.CreateDynamicMaterialInstance` (`self.Screen2`) 0 null "None"))
      (`MaterialInstanceDynamic.SetTextureParameterValue` _returnvalue_2 "BaseTexture" Tex))
    (:`2`
      (bind _returnvalue_3 (`PrimitiveComponent.CreateDynamicMaterialInstance` (`self.Screen3`) 0 null "None"))
      (`MaterialInstanceDynamic.SetTextureParameterValue` _returnvalue_3 "BaseTexture" Tex))
    (:`3`
      (bind _returnvalue_4 (`PrimitiveComponent.CreateDynamicMaterialInstance` (`self.Screen4`) 0 null "None"))
      (`MaterialInstanceDynamic.SetTextureParameterValue` _returnvalue_4 "BaseTexture" Tex))
    (:`4`
      (bind _returnvalue_5 (`PrimitiveComponent.CreateDynamicMaterialInstance` (`self.Screen5`) 0 null "None"))
      (`MaterialInstanceDynamic.SetTextureParameterValue` _returnvalue_5 "BaseTexture" Tex))
    (:`5`
      (bind _returnvalue_6 (`PrimitiveComponent.CreateDynamicMaterialInstance` (`self.Screen6`) 0 null "None"))
      (`MaterialInstanceDynamic.SetTextureParameterValue` _returnvalue_6 "BaseTexture" Tex))))

(fn `PathForIndex`
  (params (Index :type Integer))
  (returns (Path :type String))
  (switch `int` Index
    (:`Default`
      (return ""))
    (:`0`
      (return "/LoadLens/LoadLens/Assets/T_LoadLensHeavy_01.T_LoadLensHeavy_01"))
    (:`1`
      (return "/LoadLens/LoadLens/Assets/T_LoadLensHeavy_02.T_LoadLensHeavy_02"))
    (:`2`
      (return "/LoadLens/LoadLens/Assets/T_LoadLensHeavy_03.T_LoadLensHeavy_03"))
    (:`3`
      (return "/LoadLens/LoadLens/Assets/T_LoadLensHeavy_04.T_LoadLensHeavy_04"))
    (:`4`
      (return "/LoadLens/LoadLens/Assets/T_LoadLensHeavy_05.T_LoadLensHeavy_05"))
    (:`5`
      (return "/LoadLens/LoadLens/Assets/T_LoadLensHeavy_06.T_LoadLensHeavy_06"))))

(fn `UserConstructionScript`)